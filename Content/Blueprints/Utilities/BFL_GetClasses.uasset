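; Blueprint function library of shortcut getters for the project's core gameplay classes.
; Each function fetches the engine object, casts it to the project's Blueprint type and returns the typed result, covering the game state, player controller, HUD and the HUD's MainUI.
; Player controller and HUD lookups always use player index 0, and a failed cast ends the function without returning a valid reference.
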(fn `JF_GetGameState`
  (returns (`AsBP MYGame State` :type "/Game/Blueprints/Framework/BP_MyGameState Object Reference"))
  (bind _asbp_my_game_state (cast `/Game/Blueprints/Framework/BP_MyGameState` (`GameplayStatics.GetGameState` null)))
  (return _asbp_my_game_state))

(fn `JF_GetHUD`
  (returns (`AsBP My HUD` :type "/Game/Blueprints/Framework/BP_MyHUD Object Reference"))
  (bind _asbp_my_hud (cast `/Game/Blueprints/Framework/BP_MyHUD` (`PlayerController.GetHUD` (`GameplayStatics.GetPlayerController` null))))
  (return _asbp_my_hud))

(fn `JF_GetMainUI`
  (returns (`Main UI` :type "UMG_Main Object Reference"))
  (bind _asbp_my_hud (cast `/Game/Blueprints/Framework/BP_MyHUD` (`PlayerController.GetHUD` (`GameplayStatics.GetPlayerController` null))))
  (return (`MyHUD.MainUI` _asbp_my_hud)))

(fn `JF_GetPlayerController`
  (params (__WorldContext :type "Object Object Reference"))
  (returns (`AsBP Player Controller` :type "/Game/Blueprints/Framework/BP_PlayerController Object Reference"))
  (bind _asbp_player_controller (cast `/Game/Blueprints/Framework/BP_PlayerController` (`GameplayStatics.GetPlayerController` null)))
  (return _asbp_player_controller))