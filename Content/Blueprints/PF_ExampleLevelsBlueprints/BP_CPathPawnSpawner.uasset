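; Spawner actor that repeatedly creates CPath example flying pawns at random offsets around itself, each pathfinding to a destination actor and destroyed on arrival.
; A looping timer drives spawning, passing path settings and giving each pawn a random max speed.
; Every tick, it divides the cooldown by the game state's MapAP percentage for the HUD's selected AP time, clamps it, and restarts the timer when that interval changes.
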(event `self.ReceiveTick`
  (params (DeltaSeconds :type "Float (single-precision)"))
  (bind _returnvalue (/ (`BlueprintMapLibrary.Map_Find` (`MyGameState.Map_AP` (`/Game/Blueprints/Utilities/BFL_GetClasses.JF_GetGameState`)) (`KismetMathLibrary.FTrunc` (`MyHUD.ShowUser_APTime` (`/Game/Blueprints/Utilities/BFL_GetClasses.JF_GetHUD`)))) 100.0))
  (bind _returnvalue_2 (* (`KismetMathLibrary.FClamp` (/ (`self.SpawnCooldown`) (`KismetMathLibrary.SelectFloat` 0.01 _returnvalue (== _returnvalue 0.0))) 1e-05 4.0) 1.0))
  (`|ExecutionSequence`
    (:`then_0`
      (`self.CheckAndClearTimer` _returnvalue_2 (delegate `SpawnPawn`)))
    (:`then_1`
      (set `self.ValueSaved` _returnvalue_2))))

(event `SpawnPawn`
  (bind (_returnvalue_location _returnvalue_rotation _returnvalue_scale) (`KismetMathLibrary.BreakTransform` (`self.GetTransform`)))
  (bind _returnvalue (`|SpawnActorFromClass` "/Game/Blueprints/PF_ExampleLevelsBlueprints/BP_CPathExampleFlyingPawn.BP_CPathExampleFlyingPawn_C" (`KismetMathLibrary.MakeTransform` (+ (* (`KismetMathLibrary.RandomUnitVector`) (`self.RandomSpawnPosition`)) _returnvalue_location) _returnvalue_rotation _returnvalue_scale) "AdjustIfPossibleButAlwaysSpawn" "OverrideRootScale" null (0.0 0.0 0.0) (`self.DestActor`) true 0.5 (`self.DrawPaths`) (`self.Smoothing Passes`) (`self.FindPath User Data`) null))
  (`/Engine/EditorBlueprintResources/StandardMacros.IsValid` _returnvalue
    (:`Is Valid`
      (bind _flyingmovementcomponent (`/Game/Blueprints/PF_ExampleLevelsBlueprints/BP_CPathExampleFlyingPawn.FlyingMovementComponent` _returnvalue))
      (`/Engine/EditorBlueprintResources/StandardMacros.IsValid` _flyingmovementcomponent
        (:`Is Valid`
          (set `FloatingPawnMovement.MaxSpeed` (`KismetMathLibrary.RandomFloatInRange` (`self.MinSpeed`) (`self.MaxSpeed`)) _flyingmovementcomponent))))))

(event `self.ReceiveBeginPlay`
  (`KismetSystemLibrary.Delay` (`self.ValueSaved`))
  (bind _returnvalue (`KismetSystemLibrary.K2_SetTimerDelegate` (delegate `SpawnPawn`) 1.0 true))
  (set `self.TH_SpawnCpathPawn` _returnvalue))

(fn `CheckAndClearTimer`
  (params (InputPin :type "Float (double-precision)") (Event :type Delegate))
  (if (!= (`self.ValueSaved`) InputPin)
    (set `self.ValueSaved` InputPin)
    (`KismetSystemLibrary.K2_ClearAndInvalidateTimerHandle` (`self.TH_SpawnCpathPawn`))
    (bind _returnvalue (`KismetSystemLibrary.K2_SetTimerDelegate` Event InputPin true))
    (set `self.TH_SpawnCpathPawn` _returnvalue)))

(fn `UserConstructionScript`)