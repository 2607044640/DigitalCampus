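; Spawner actor for the CPath example levels that periodically creates flying example pawns at its own transform.
; A looping timer started on BeginPlay spawns each BP_CPathExampleFlyingPawn with a destination actor, path smoothing, debug drawing and pathfinding user data passed in at spawn.
; Each pawn is set to destroy itself on arrival and gets a random flying max speed within a configured range.
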(event `self.ReceiveBeginPlay`
  (`KismetSystemLibrary.K2_SetTimerDelegate` (delegate `Spawn`) (`self.SpawnCooldown`) true (`self.InitialDelay`)))

(event `Spawn`
  (bind _returnvalue (`|SpawnActorFromClass` "/CPathfinding/Blueprints/ExampleLevelsBlueprints/BP_CPathExampleFlyingPawn.BP_CPathExampleFlyingPawn_C" (`self.GetTransform`) "AlwaysSpawn" "OverrideRootScale" null (0.0 0.0 0.0) (`self.DestActor`) true 0.5 (`self.DrawPaths`) (`self.Smoothing Passes`) (`self.FindPath User Data`) null))
  (set `FloatingPawnMovement.MaxSpeed` (`KismetMathLibrary.RandomFloatInRange` (`self.MinSpeed`) (`self.MaxSpeed`)) (`/CPathfinding/Blueprints/ExampleLevelsBlueprints/BP_CPathExampleFlyingPawn.FlyingMovementComponent` _returnvalue)))

(fn `UserConstructionScript`)