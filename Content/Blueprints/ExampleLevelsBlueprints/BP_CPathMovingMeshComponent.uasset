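; Example-level component that moves its owning actor back and forth between the actor's starting location and the component's own starting world location.
; BeginPlay records both endpoints and starts a timer that calls Update at a set rate, with a randomized initial delay, instead of using Tick.
; Update eases the actor toward the current target with teleport-free, unswept location sets.
; On arrival, a FlipFlop swaps the target and CalculateDelay sets the pause before the next move.
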(event `self.ReceiveBeginPlay`
  ;[1 1 1] Begin Play, Initializing timer
  (bind _output_get (set `self.OwningActor` (`self.GetOwner`)))
  (set `self.InitialActorLocation` (`Actor.K2_GetActorLocation` _output_get))
  (set `self.InitialComponentLocation` (`self.K2_GetComponentLocation`))
  (`self.SetNewTarget`)
  (`KismetSystemLibrary.K2_SetTimerDelegate` (delegate `Update`) (`self.UpdateRate`) (`self.bLoop`) (`self.InitialDelay`) (`self.RandomDelayDeviation`)))

(event `Update`
  (bind _randomdelaydeviation (`self.RandomDelayDeviation`))
  ;[1 1 1] Moving the actor to target or waiting for next loop
  (if (<= (`self.TimeTillNextMove`) 0.0)
    (`Actor.K2_SetActorLocation` (`self.OwningActor`) (`|EaseFunction` "EaseOut" (/ (`self.CurrMoveTime`) (`self.MoveDuration`)) (`KismetMathLibrary.SelectVector` (`self.InitialComponentLocation`) (`self.InitialActorLocation`) (== (`self.CurrTarget`) (`self.InitialActorLocation`) :`ErrorTolerance` 0.005)) (`self.CurrTarget`)) false false)
    (if (`KismetMathLibrary.NearlyEqual_FloatFloat` (/ (`self.CurrMoveTime`) (`self.MoveDuration`)) 1.0 0.005)
      (`self.SetNewTarget`)
      (set `self.TimeTillNextMove` (+ (`self.LoopingDelay`) (`KismetMathLibrary.RandomFloatInRange` (* _randomdelaydeviation -1.0) _randomdelaydeviation)))
      (set `self.CurrMoveTime` 0.0)
      (else
        (set `self.CurrMoveTime` (+ (`self.CurrMoveTime`) (`self.UpdateRate`)))))
    (else
      (set `self.TimeTillNextMove` (- (`self.TimeTillNextMove`) (`self.UpdateRate`))))))

(event `SetNewTarget`
  ;[1 1 1] Toggle target between initial actor location and this component's location
  (`/Engine/EditorBlueprintResources/StandardMacros.FlipFlop`
    (:`A`
      (set `self.CurrTarget` (`self.InitialComponentLocation`)))
    (:`B`
      (set `self.CurrTarget` (`self.InitialActorLocation`)))))